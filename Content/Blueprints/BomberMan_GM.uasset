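; BomberMan game mode that runs the match countdown and tracks how many enemies remain.
; Tick uses a one-second Delay as a timer to decrement Minutes and Seconds, then at zero shows TimeOverScreen with the mouse cursor and pauses the game.
; Events increment or decrement the enemy count, and a separate check sets EnemiesDied when none remain.
; The RepNotify functions and the CheckEnemies, DecrementEnemies and IncrementEnemies events are empty.
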(event `self.ReceiveTick`
  (params (DeltaSeconds :type "Float (single-precision)"))
  (`KismetSystemLibrary.Delay` 1.0)
  (if (== (`self.Seconds`) 0)
    (if (== (`self.Minutes`) 0)
      (bind _returnvalue (`|CreateWidget` "/Game/UMG/UI/TimeOverScreen.TimeOverScreen_C"))
      (`UserWidget.AddToViewport` _returnvalue 0)
      (set `PlayerController.bShowMouseCursor` true (`GameplayStatics.GetPlayerController` 0))
      (`GameplayStatics.SetGamePaused` true)
      (else
        (set `self.Seconds` 59)
        (set `self.Minutes` (- (`self.Minutes`) 1))))
    (else
      (set `self.Seconds` (- (`self.Seconds`) 1)))))

(event `Check No of Enemies`
  (if (<= (`self.Number of Enemies`) 0)
    (set `self.Enemies Died` true)
    (else
      (set `self.Enemies Died` false))))

(event `/Game/Interface/CheckNoOfEnemies.Check Enemies`)

(event `Decrement No of Enemy`
  (set `self.Number of Enemies` (- (`self.Number of Enemies`) 1)))

(event `/Game/Interface/DecrementNoOfEnemies.Decrement Enemies`)

(event `Increment No of Enemy`
  (set `self.Number of Enemies` (+ (`self.Number of Enemies`) 1)))

(event `/Game/Interface/IncrementNoOfEnemies.Increment Enemies`)

(fn `OnRep_Minutes`)

(fn `OnRep_Number of Enemies`)

(fn `OnRep_Total Kill Count`)

(fn `UserConstructionScript`)