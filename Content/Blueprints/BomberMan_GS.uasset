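; BomberMan game state Blueprint that provides a shared area-of-effect hit function, SpawnAOE.
; SpawnAOE temporarily binds the caller's event to the AOEHit dispatcher, fires it for each Pawn in a sphere overlap, then unbinds it.
; The instigator is excluded from the overlap.
; The LOS input is unused, the debug sphere drawing is disconnected, and the event graph is empty.
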(event `self.ReceiveBeginPlay`)

(fn `Spawn AOE`
  (params (Location :type "Vector Structure") (Radius :type "Float (double-precision)") (LOS :type Boolean) (Instigator :type "Actor Object Reference") (`Hit Event` :type "Delegate (by ref)") (`Debug Duration` :type "Float (double-precision)") (`Debug Color` :type "LinearColor Structure"))
  (set `self.Debug Color_0` `Debug Color`)
  (add `self.AOE Hit` `Hit Event`)
  (`|ExecutionSequence`
    (:`then_0`
      (bind _outactors (`KismetSystemLibrary.SphereOverlapActors` (`local.Location`) (`local.Radius`) (`|MakeArray` "ObjectTypeQuery3" :!type "EObjectTypeQuery Enum") null (`|MakeArray` (`local.Instigator`))))
      (for _array_element _outactors
        (bind _output_get (set `self.Current Actor` _array_element))
        (`self.AOE Hit` _output_get)))
    (:`then_1`
      (remove `self.AOE Hit` (`local.Hit Event`)))))

(fn `UserConstructionScript`)