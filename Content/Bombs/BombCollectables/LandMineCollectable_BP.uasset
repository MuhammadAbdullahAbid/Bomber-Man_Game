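; Land mine pickup that grows in through a scale timeline on BeginPlay and caches the player character.
; When the player or a Collector AI overlaps its box, it destroys itself and credits the player with two land mines, capped at two.
; Collection also zeroes the player's other bomb counts and clears the box package flag, so land mines replace those bombs.
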(event `self.ReceiveBeginPlay`
  (bind _asthird_person_character (cast `/Game/ThirdPersonCPP/Blueprints/ThirdPersonCharacter` (`GameplayStatics.GetPlayerCharacter` 0)))
  (set `self.As Third Person Character` _asthird_person_character)
  (bind (_direction _scale) (`Timeline|Scale` :!via `PlayFromStart`)
    (:`Update`
      (`SceneComponent.SetWorldScale3D` (`self.StaticMesh`) (`KismetMathLibrary.Conv_DoubleToVector` (* _scale 15.0))))))

(event `self.Box.OnComponentBeginOverlap`
  (params (OverlappedComponent :type "PrimitiveComponent Object Reference") (OtherActor :type "Actor Object Reference") (OtherComp :type "PrimitiveComponent Object Reference") (OtherBodyIndex :type Integer) (bFromSweep :type Boolean) (SweepResult :type "HitResult Structure (by ref)"))
  (bind _as_third_person_character (`self.As Third Person Character`))
  (bind _as_third_person_character_2 (`self.As Third Person Character`))
  (bind _returnvalue (+ (`Bomber_ManCharacter.LandMine` _as_third_person_character_2) 2))
  (cast `/Game/AI/Collector/Collector_AI_BP` OtherActor
    (:`then`
      (`self.K2_DestroyActor` :!label _label)
      (if (> _returnvalue 2)
        (set `Bomber_ManCharacter.LandMine` 2 _as_third_person_character_2)
        (else
          (set `Bomber_ManCharacter.LandMine` _returnvalue _as_third_person_character_2)))
      (set `Bomber_ManCharacter.BasicTimeBomb` 0 _as_third_person_character)
      (set `Bomber_ManCharacter.StickyBomb` 0 _as_third_person_character)
      (set `Bomber_ManCharacter.InvertBomb` 0 _as_third_person_character)
      (set `Bomber_ManCharacter.FreezeBomb` 0 _as_third_person_character)
      (set `Bomber_ManCharacter.InstantBomb` 0 _as_third_person_character)
      (set `Bomber_ManCharacter.isBoxPackage` false _as_third_person_character))
    (:`CastFailed`
      (if (== OtherActor (`self.As Third Person Character`))
        (goto _label)))))

(fn `UserConstructionScript`)