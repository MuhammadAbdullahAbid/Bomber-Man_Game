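; Collectable pickup that gives the player Invert Bombs.
; When the player pawn overlaps its sphere, the actor destroys itself and adds to the ThirdPersonCharacter's InvertBomb count.
; It also zeroes the other bomb type counts and clears the IsBoxPackage flag, so the pickup replaces any other held bomb type.
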(event `self.Sphere.OnComponentBeginOverlap`
  (params (OverlappedComponent :type "PrimitiveComponent Object Reference") (OtherActor :type "Actor Object Reference") (OtherComp :type "PrimitiveComponent Object Reference") (OtherBodyIndex :type Integer) (bFromSweep :type Boolean) (SweepResult :type "HitResult Structure (by ref)"))
  (bind _as_third_person_character (`self.As Third Person Character`))
  (if (== OtherActor (`GameplayStatics.GetPlayerPawn` 0))
    (`self.K2_DestroyActor`)
    (bind _asthird_person_character (cast `/Game/ThirdPersonCPP/Blueprints/ThirdPersonCharacter` (`GameplayStatics.GetPlayerCharacter` 0)))
    (bind _output_get (set `self.As Third Person Character` _asthird_person_character))
    (set `Bomber_ManCharacter.InvertBomb` (+ (`Bomber_ManCharacter.InvertBomb` _output_get) 2) _output_get)
    (set `Bomber_ManCharacter.BasicTimeBomb` 0 _as_third_person_character)
    (set `Bomber_ManCharacter.LandMine` 0 _as_third_person_character)
    (set `Bomber_ManCharacter.InstantBomb` 0 _as_third_person_character)
    (set `Bomber_ManCharacter.FreezeBomb` 0 _as_third_person_character)
    (set `Bomber_ManCharacter.StickyBomb` 0 _as_third_person_character)
    (set `Bomber_ManCharacter.isBoxPackage` false _as_third_person_character)))

(fn `UserConstructionScript`)