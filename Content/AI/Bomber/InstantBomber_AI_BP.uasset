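; Instant bomber AI character Blueprint whose only scripted behavior is a reaction to a freeze attack.
; FreezeAttack sets a StopAction flag, pauses mesh animation, disables movement and applies an ice material.
; After a fixed delay it clears the flag, resumes animation, restores walking and sets a pulsing hex-tile material.
; A DoOnce gate, reset on thaw, blocks overlapping freezes.
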(event `/Game/Bombs/FreezeDamageInteface.FreezeAttack`
  ;[0 0.3055 1] Freeze Attack
  (`/Engine/EditorBlueprintResources/StandardMacros.DoOnce` false :!label _label
    (:`Completed`
      (set `self.StopAction` true)
      (set `SkeletalMeshComponent.bPauseAnims` true (`self.Mesh`))
      (`CharacterMovementComponent.DisableMovement` (`self.CharacterMovement`))
      (`PrimitiveComponent.SetMaterial` (`self.Mesh`) 0 "/Game/Materials/ice_Mat_Inst.ice_Mat_Inst")
      (`KismetSystemLibrary.Delay` 4.0)
      (set `self.StopAction` false)
      (set `SkeletalMeshComponent.bPauseAnims` false (`self.Mesh`))
      (`PrimitiveComponent.SetMaterial` (`self.Mesh`) 0 "/Game/StarterContent/Materials/M_Tech_Hex_Tile_Pulse.M_Tech_Hex_Tile_Pulse")
      (`CharacterMovementComponent.SetMovementMode` (`self.CharacterMovement`) "MOVE_Walking" 0)
      (goto _label :!via `Reset`))))

(fn `UserConstructionScript`
  (`parent.UserConstructionScript`))