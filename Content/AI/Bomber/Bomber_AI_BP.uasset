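; Bomber enemy character that chases the player, throws time bombs and reports its death to BomberMan_GM.
; BeginPlay links it to its AI controller and health bar widget, and MoveToPlayer runs a repeating AIMoveTo.
; Spawning attaches a bomb to the mesh socket, and Throwing releases it forward with physics.
; AnyDamage drives health-bar fade, blood and ragdoll death, while FreezeAttack temporarily halts movement, animation and AI under an ice material.
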(event `self.ReceiveBeginPlay`
  (bind _asthird_person_character (cast `/Game/ThirdPersonCPP/Blueprints/ThirdPersonCharacter` (`GameplayStatics.GetPlayerCharacter` 0)))
  (set `self.As Third Person Character` _asthird_person_character)
  (bind _asbomber_man_gm (cast `/Game/Blueprints/BomberMan_GM` (`GameplayStatics.GetGameMode`)))
  (set `self.As Bomber Man GM` _asbomber_man_gm)
  (bind _asbomber_health_bar (cast `/Game/UMG/HealthBars/BomberHealthBar` (`WidgetComponent.GetWidget` (`self.Widget`))))
  (bind _output_get (set `self.As Bomber Health Bar` _asbomber_health_bar))
  (set `/Game/UMG/HealthBars/BomberHealthBar.Bomber AI BP` self _output_get)
  (bind _asmy_enemy_aicontroller_bomber_bp (cast `/Game/AI/Bomber/MyEnemy_AIControllerBomberBP` (`self.GetController`)))
  (set `self.As My Enemy AIController Bomber BP` _asmy_enemy_aicontroller_bomber_bp)
  (set `/Game/AI/Bomber/MyEnemy_AIControllerBomberBP.Bomber AI BP` self _asmy_enemy_aicontroller_bomber_bp))

(event `Move To Player`
  (params (AcceptanceRadius :type "Float (double-precision)"))
  ;[0.02577 0.1042 0] AI MoveTO
  (`/Engine/EditorBlueprintResources/StandardMacros.IsValid` (`self.As Third Person Character`) :!label _label
    (:`Is Valid`
      (`|AIMoveTo` self (100.0 50.0 0.0) (`self.As Third Person Character`) AcceptanceRadius
        (:`OnSuccess`
          (`KismetSystemLibrary.Delay` 3.0)
          (goto _label))
        (:`OnFail`
          (goto _label))))
    (:`Is Not Valid`
      (`KismetSystemLibrary.Delay` 1.0)
      (goto _label))))

(event `self.ReceiveAnyDamage`
  (params (Damage :type "Float (single-precision)") (DamageType :type "DamageType Object Reference") (InstigatedBy :type "Controller Object Reference") (DamageCauser :type "Actor Object Reference"))
  (bind _as_bomber_health_bar (`self.As Bomber Health Bar`))
  (bind _as_bomber_man_gm (`self.As Bomber Man GM`))
  (`|ExecutionSequence`
    (:`then_0`
      ;[0.08333 0.00304 0] Death Condition
      (if (== (`YTHealthComponent.Health` (`self.YTHealth`)) 0.0)
        (`PrimitiveComponent.SetSimulatePhysics` (`self.Mesh`) true)
        (`CharacterMovementComponent.DisableMovement` (`self.CharacterMovement`))
        (`self.DetachFromControllerPendingDestroy`)
        (`|ExecutionSequence`
          (:`then_0`
            (`ActorComponent.K2_DestroyComponent` (`self.CapsuleComponent`))
            (`ActorComponent.K2_DestroyComponent` (`self.Widget`)))
          (:`then_1`
            (`KismetSystemLibrary.Delay` 1.56)
            (`/Engine/EditorBlueprintResources/StandardMacros.IncrementInt` (`/Game/Blueprints/BomberMan_GM.Total Kill Count` (`self.As Bomber Man GM`))
              (:`  `
                (`/Game/Blueprints/BomberMan_GM.Decrement No of Enemy` _as_bomber_man_gm)
                (`/Game/Blueprints/BomberMan_GM.Check No of Enemies` _as_bomber_man_gm)
                (`SceneComponent.K2_DetachFromComponent` (`self.Mesh`) "KeepWorld" "KeepWorld" "KeepWorld" true)
                (`self.K2_DestroyActor`)))))))
    (:`then_1`
      (`UserWidget.PlayAnimation` _as_bomber_health_bar (`/Game/UMG/HealthBars/BomberHealthBar.HeathFade` _as_bomber_health_bar) 0.0 1 "Forward" 1.0 true))
    (:`then_2`
      (`NiagaraFunctionLibrary.SpawnSystemAtLocation` "/Game/Particles/BloodSplash02.BloodSplash02" (`SceneComponent.GetSocketLocation` (`self.Mesh`) "neck_01")))))

(event `Freeze Bomb Attack`)

(event `/Game/Bombs/FreezeDamageInteface.FreezeAttack`
  ;[0 0.3055 1] Freeze Attack
  (`/Engine/EditorBlueprintResources/StandardMacros.DoOnce` false :!label _label_2
    (:`Completed`
      (set `/Game/AI/Bomber/MyEnemy_AIControllerBomberBP.Stop` true (`self.As My Enemy AIController Bomber BP`))
      (set `self.StopAction` true)
      (set `SkeletalMeshComponent.bPauseAnims` true (`self.Mesh`))
      (`CharacterMovementComponent.DisableMovement` (`self.CharacterMovement`))
      (`PrimitiveComponent.SetMaterial` (`self.Mesh`) 0 "/Game/Materials/ice_Mat_Inst.ice_Mat_Inst")
      (`KismetSystemLibrary.Delay` 4.0)
      (set `/Game/AI/Bomber/MyEnemy_AIControllerBomberBP.Stop` false (`self.As My Enemy AIController Bomber BP`))
      (set `self.StopAction` false)
      (set `SkeletalMeshComponent.bPauseAnims` false (`self.Mesh`))
      (`PrimitiveComponent.SetMaterial` (`self.Mesh`) 0 "/Game/StarterContent/Materials/M_Metal_Steel.M_Metal_Steel")
      (`CharacterMovementComponent.SetMovementMode` (`self.CharacterMovement`) "MOVE_Walking" 0)
      (goto _label_2 :!via `Reset`))))

(event `Spawning`
  (bind _returnvalue (`|SpawnActorFromClass` "/Game/Bombs/BombTest/TestTimeBomb.TestTimeBomb_C" (`SceneComponent.K2_GetComponentToWorld` (`self.Arrow1`)) "Undefined" "OverrideRootScale" null null))
  (`self.K2_AttachToComponent` _returnvalue (`self.Mesh`) "BombAttachment" "KeepWorld" "KeepWorld" "KeepWorld" true))

(event `Throwing`
  (`self.K2_DetachFromActor` (stale `Spawning` _returnvalue) "KeepWorld" "KeepWorld" "KeepWorld")
  (bind _staticmesh (`/Game/Bombs/BombTest/TestTimeBomb.StaticMesh` (stale `Spawning` _returnvalue)))
  (`PrimitiveComponent.SetSimulatePhysics` _staticmesh true)
  (`PrimitiveComponent.SetPhysicsLinearVelocity` _staticmesh (* (`self.GetActorForwardVector`) 1000.0) false "None"))

(fn `OnRep_As Bomber Man GM`)

(fn `UserConstructionScript`)