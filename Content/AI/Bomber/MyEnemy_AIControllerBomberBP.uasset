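; AI controller for the Bomber enemy that starts its behavior tree and drives a repeating bomb attack.
; After BeginPlay runs Bomber_BT, an endless Delay loop alternates spawning and throwing a bomb through BomberAIBP, three seconds apart.
; A Stop flag, not set in this graph, gates both actions without breaking the loop.
; Some debug and older spawn/throw calls remain disconnected.
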(event `self.ReceiveBeginPlay`
  (`self.RunBehaviorTree` "/Game/AI/Bomber/Bomber_BT.Bomber_BT")
  (`self.SpawnAndThrow` :!label _label)
  (`KismetSystemLibrary.Delay` 3.0)
  (`self.Throw`)
  (`KismetSystemLibrary.Delay` 3.0)
  (goto _label))

(event `SpawnAndThrow`
  (if (not (`self.Stop`))
    (`Bomber_AI.SpawnBomb` (`self.Bomber AI BP`))))

(event `Throw`
  (if (not (`self.Stop`))
    (`Bomber_AI.ThrowBomb` (`self.Bomber AI BP`))))

(fn `UserConstructionScript`)