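; Collector enemy character for a Bomberman game that chases bomb collectables around the level.
; Roughly every second, Tick picks a random collectable class and issues AIMoveTo toward each of its actors.
; Damage fades the health bar widget and spawns blood; at zero health it ragdolls, updates GameMode kill and enemy counts, then destroys itself.
; FreezeAttack temporarily halts animation and movement with an ice material, guarded by a DoOnce.
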(event `self.ReceiveTick`
  (params (DeltaSeconds :type "Float (single-precision)"))
  (`KismetSystemLibrary.Delay` 1.0)
  (bind _outactors (`GameplayStatics.GetAllActorsOfClass` (select `int` (`KismetMathLibrary.RandomIntegerInRange` 0 4) :`0` "/Game/Bombs/BombCollectables/BasicTimeBombCollectable_BP.BasicTimeBombCollectable_BP_C" :`1` "/Game/Bombs/BombCollectables/InstantBombCollectable_BP.InstantBombCollectable_BP_C" :`2` "/Game/Bombs/BombCollectables/LandMineCollectable_BP.LandMineCollectable_BP_C" :`3` "/Game/Bombs/BombCollectables/StickyBombCollectable_BP.StickyBombCollectable_BP_C" :`4` "/Game/Bombs/BombCollectables/FreezeBombCollectable_BP.FreezeBombCollectable_BP_C" :!type "Actor Class Reference")))
  (for _array_element _outactors
    (`|AIMoveTo` self (`self.K2_GetActorLocation` _array_element) _array_element 1.0)))

(event `self.ReceiveBeginPlay`
  (bind _asbomber_man_gm (cast `/Game/Blueprints/BomberMan_GM` (`GameplayStatics.GetGameMode`)))
  (set `self.As Bomber Man GM` _asbomber_man_gm)
  (bind _ascollector_ai_controller_bp (cast `/Game/AI/Collector/CollectorAI_ControllerBP` (`self.GetController`)))
  (set `/Game/AI/Collector/CollectorAI_ControllerBP.Collector_AI_BP` self _ascollector_ai_controller_bp)
  (bind _ascollector_health_bar (cast `/Game/UMG/HealthBars/CollectorHealthBar` (`WidgetComponent.GetWidget` (`self.Widget`))))
  (set `self.As Collector Health Bar` _ascollector_health_bar)
  (set `/Game/UMG/HealthBars/CollectorHealthBar.Collector AI BP` self _ascollector_health_bar))

(event `self.ReceiveAnyDamage`
  (params (Damage :type "Float (single-precision)") (DamageType :type "DamageType Object Reference") (InstigatedBy :type "Controller Object Reference") (DamageCauser :type "Actor Object Reference"))
  (bind _as_bomber_man_gm (`self.As Bomber Man GM`))
  (bind _as_collector_health_bar (`self.As Collector Health Bar`))
  (`|ExecutionSequence`
    (:`then_0`
      ;[0.08333 0.00304 0] Death Condition
      (if (== (`YTHealthComponent.Health` (`self.YTHealth`)) 0.0)
        (`PrimitiveComponent.SetSimulatePhysics` (`self.Mesh`) true)
        (`CharacterMovementComponent.DisableMovement` (`self.CharacterMovement`))
        (`self.DetachFromControllerPendingDestroy`)
        (`ActorComponent.K2_DestroyComponent` (`self.CapsuleComponent`))
        (`ActorComponent.K2_DestroyComponent` (`self.Widget`))
        (`KismetSystemLibrary.Delay` 2.0)
        (`/Engine/EditorBlueprintResources/StandardMacros.IncrementInt` (`/Game/Blueprints/BomberMan_GM.Total Kill Count` _as_bomber_man_gm)
          (:`  `
            (`/Game/Blueprints/BomberMan_GM.Decrement No of Enemy` _as_bomber_man_gm)
            (`/Game/Blueprints/BomberMan_GM.Check No of Enemies` _as_bomber_man_gm)
            (`self.K2_DestroyActor`)))))
    (:`then_1`
      (`UserWidget.PlayAnimation` _as_collector_health_bar (`/Game/UMG/HealthBars/CollectorHealthBar.HeathFade` _as_collector_health_bar) 0.0 1 "Forward" 1.0 true))
    (:`then_2`
      (`NiagaraFunctionLibrary.SpawnSystemAtLocation` "/Game/Particles/BloodSplash02.BloodSplash02" (`SceneComponent.GetSocketLocation` (`self.Mesh`) "neck_01")))))

(event `/Game/Bombs/FreezeDamageInteface.FreezeAttack`
  ;[0 0.3055 1] Freeze Attack
  (`/Engine/EditorBlueprintResources/StandardMacros.DoOnce` false :!label _label
    (:`Completed`
      (set `SkeletalMeshComponent.bPauseAnims` true (`self.Mesh`))
      (`CharacterMovementComponent.DisableMovement` (`self.CharacterMovement`))
      (`PrimitiveComponent.SetMaterial` (`self.Mesh`) 0 "/Game/Materials/ice_Mat_Inst.ice_Mat_Inst")
      (`KismetSystemLibrary.Delay` 4.0)
      (set `SkeletalMeshComponent.bPauseAnims` false (`self.Mesh`))
      (`PrimitiveComponent.SetMaterial` (`self.Mesh`) 0 "/Game/Mannequin/Character/Materials/MI_Female_Body.MI_Female_Body")
      (`CharacterMovementComponent.SetMovementMode` (`self.CharacterMovement`) "MOVE_Walking" 0)
      (goto _label :!via `Reset`))))

(fn `OnRep_As Collector Health Bar`)

(fn `UserConstructionScript`)