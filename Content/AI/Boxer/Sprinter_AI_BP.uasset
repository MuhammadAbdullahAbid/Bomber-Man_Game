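; Sprinter AI character Blueprint that can be temporarily frozen by a freeze attack.
; FreezeAttack pauses mesh animation, disables movement and applies an ice material, then after a short delay resumes animation, sets a cobblestone material and restores walking.
; A DoOnce gate ignores repeat freezes until the current one ends.
; The FreezeBomb event is empty, and the file contains no other AI logic.
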(event `Freeze Bomb`)

(event `/Game/Bombs/FreezeDamageInteface.FreezeAttack`
  (`/Engine/EditorBlueprintResources/StandardMacros.DoOnce` false :!label _label
    (:`Completed`
      (set `SkeletalMeshComponent.bPauseAnims` true (`self.Mesh`))
      (`CharacterMovementComponent.DisableMovement` (`self.CharacterMovement`))
      (`PrimitiveComponent.SetMaterial` (`self.Mesh`) 0 "/Game/Materials/ice_Mat_Inst.ice_Mat_Inst")
      (`KismetSystemLibrary.Delay` 4.0)
      (set `SkeletalMeshComponent.bPauseAnims` false (`self.Mesh`))
      (`PrimitiveComponent.SetMaterial` (`self.Mesh`) 0 "/Game/StarterContent/Materials/M_CobbleStone_Pebble.M_CobbleStone_Pebble")
      (`CharacterMovementComponent.SetMovementMode` (`self.CharacterMovement`) "MOVE_Walking" 0)
      (goto _label :!via `Reset`))))

(fn `UserConstructionScript`
  (`parent.UserConstructionScript`))