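; Boxer enemy character for the BomberMan game mode, linked to its AI controller and health bar widget on BeginPlay.
; MoveToPlayer repeatedly chases the player, while Punch, Attack and FreezeBombAttack are empty.
; Damage fades the health bar and spawns blood; at zero health it ragdolls, updates game-mode kill and enemy counts, then destroys itself.
; FreezeAttack uses a DoOnce to temporarily halt controller, animation and movement with an ice material.
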(event `Punch`
  ;[1 0 0.2172] Punching
)

(event `Move To Player`
  (params (AcceptanceRadius :type "Float (double-precision)"))
  ;[0.02577 0.1042 0] AI MoveTO
  (`/Engine/EditorBlueprintResources/StandardMacros.IsValid` (`self.As Third Person Character`) :!label _label
    (:`Is Valid`
      (`|AIMoveTo` self (100.0 50.0 0.0) (`self.As Third Person Character`) AcceptanceRadius
        (:`OnSuccess`
          (`KismetSystemLibrary.Delay` 3.0)
          (goto _label))))
    (:`Is Not Valid`
      (`KismetSystemLibrary.Delay` 1.0)
      (goto _label))))

(event `self.ReceiveBeginPlay`
  ;[0.09375 0.09375 0.09375] BeginPlay
  (bind _asthird_person_character (cast `/Game/ThirdPersonCPP/Blueprints/ThirdPersonCharacter` (`GameplayStatics.GetPlayerCharacter` 0)))
  (set `self.As Third Person Character` _asthird_person_character)
  (bind _asbomber_man_gm (cast `/Game/Blueprints/BomberMan_GM` (`GameplayStatics.GetGameMode`)))
  (set `self.As Bomber Man GM` _asbomber_man_gm)
  (bind _asboxer_health_bar (cast `/Game/UMG/HealthBars/BoxerHealthBar` (`WidgetComponent.GetWidget` (`self.Widget`))))
  (bind _output_get (set `self.As Boxer Health Bar` _asboxer_health_bar))
  (set `/Game/UMG/HealthBars/BoxerHealthBar.Boxer AI BP` self _output_get)
  (bind _asmy_enemy_aicontroller_bp (cast `/Game/AI/Boxer/MyEnemy_AIController_BP` (`self.GetController`)))
  (set `self.As My Enemy AIController BP` _asmy_enemy_aicontroller_bp)
  (set `/Game/AI/Boxer/MyEnemy_AIController_BP.Boxer AI BP` self _asmy_enemy_aicontroller_bp))

(event `Attack`)

(event `self.ReceiveAnyDamage`
  (params (Damage :type "Float (single-precision)") (DamageType :type "DamageType Object Reference") (InstigatedBy :type "Controller Object Reference") (DamageCauser :type "Actor Object Reference"))
  (bind _as_bomber_man_gm (`self.As Bomber Man GM`))
  (bind _as_boxer_health_bar (`self.As Boxer Health Bar`))
  (`|ExecutionSequence`
    (:`then_0`
      ;[0.08333 0.00304 0] Death Condition
      (if (== (`YTHealthComponent.Health` (`self.YTHealth`)) 0.0)
        (`PrimitiveComponent.SetSimulatePhysics` (`self.Mesh`) true)
        (`CharacterMovementComponent.DisableMovement` (`self.CharacterMovement`))
        (`self.DetachFromControllerPendingDestroy`)
        (`|ExecutionSequence`
          (:`then_0`
            (`ActorComponent.K2_DestroyComponent` (`self.CapsuleComponent`))
            (`ActorComponent.K2_DestroyComponent` (`self.Widget`)))
          (:`then_1`
            (`KismetSystemLibrary.Delay` 1.5)
            (`/Engine/EditorBlueprintResources/StandardMacros.IncrementInt` (`/Game/Blueprints/BomberMan_GM.Total Kill Count` _as_bomber_man_gm)
              (:`  `
                (`/Game/Blueprints/BomberMan_GM.Decrement No of Enemy` _as_bomber_man_gm)
                (`/Game/Blueprints/BomberMan_GM.Check No of Enemies` _as_bomber_man_gm)
                (`self.K2_DestroyActor`)))))))
    (:`then_1`
      (`UserWidget.PlayAnimation` _as_boxer_health_bar (`/Game/UMG/HealthBars/BoxerHealthBar.HealthFade` _as_boxer_health_bar) 0.0 1 "Forward" 1.0 true))
    (:`then_2`
      (`NiagaraFunctionLibrary.SpawnSystemAtLocation` "/Game/Particles/BloodSplash02.BloodSplash02" (`SceneComponent.GetSocketLocation` (`self.Mesh`) "neck_01")))))

(event `Freeze Bomb Attack`)

(event `/Game/Bombs/FreezeDamageInteface.FreezeAttack`
  ;[0 0.3055 1] Freeze Attack
  (`/Engine/EditorBlueprintResources/StandardMacros.DoOnce` false :!label _label_2
    (:`Completed`
      (set `/Game/AI/Boxer/MyEnemy_AIController_BP.Stop` true (`self.As My Enemy AIController BP`))
      (set `SkeletalMeshComponent.bPauseAnims` true (`self.Mesh`))
      (`CharacterMovementComponent.DisableMovement` (`self.CharacterMovement`))
      (`PrimitiveComponent.SetMaterial` (`self.Mesh`) 0 "/Game/Materials/ice_Mat_Inst.ice_Mat_Inst")
      (`KismetSystemLibrary.Delay` 4.0)
      (set `/Game/AI/Boxer/MyEnemy_AIController_BP.Stop` false (`self.As My Enemy AIController BP`))
      (set `SkeletalMeshComponent.bPauseAnims` false (`self.Mesh`))
      (`PrimitiveComponent.SetMaterial` (`self.Mesh`) 0 "/Game/StarterContent/Materials/M_Wood_Oak.M_Wood_Oak")
      (`CharacterMovementComponent.SetMovementMode` (`self.CharacterMovement`) "MOVE_Walking" 0)
      (goto _label_2 :!via `Reset`))))

(event `self.PickUpRange.OnComponentBeginOverlap`
  (params (OverlappedComponent :type "PrimitiveComponent Object Reference") (OtherActor :type "Actor Object Reference") (OtherComp :type "PrimitiveComponent Object Reference") (OtherBodyIndex :type Integer) (bFromSweep :type Boolean) (SweepResult :type "HitResult Structure (by ref)"))
  (if (== OtherActor (`GameplayStatics.GetPlayerCharacter` 0))
    (set `self.IsinPickUpRange` true)))

(fn `UserConstructionScript`)